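; Runner track tile for level 2 that fills its three lanes with obstacles or gems and extends the track.
; On BeginPlay, SpawnObstacles randomly leaves Lane0 empty or spawns an obstacle or gem, rolling each following lane only after an obstacle.
; When ThirdPersonCharacter2 overlaps the Box, ThirdPersonGameModeLevel2 spawns the next tile.
; The points increment and delayed self-destroy logic are disconnected, so they never run.
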(event `self.ReceiveBeginPlay`
  (`self.SpawnObstacles`))

(event `self.Box.OnComponentBeginOverlap`
  (params (OverlappedComponent :type "PrimitiveComponent Object Reference") (OtherActor :type "Actor Object Reference") (OtherComp :type "PrimitiveComponent Object Reference") (OtherBodyIndex :type Integer) (bFromSweep :type Boolean) (SweepResult :type "HitResult Structure (by ref)"))
  (cast `/Game/ThirdPersonBP/Blueprints/ThirdPersonCharacter2` OtherActor)
  (bind _asthird_person_game_mode_level_2 (cast `/Game/ThirdPersonBP/Blueprints/ThirdPersonGameModeLevel2` (`GameplayStatics.GetGameMode`)))
  (`/Game/ThirdPersonBP/Blueprints/ThirdPersonGameModeLevel2.Spawn Tile` _asthird_person_game_mode_level_2)
  (bind _asthird_person_game_mode_level_2_2 (cast `/Game/ThirdPersonBP/Blueprints/ThirdPersonGameModeLevel2` (`GameplayStatics.GetGameMode`))))

(fn `SpawnObstacles`
  (bind _returnvalue (`SceneComponent.K2_GetComponentToWorld` (`self.Lane2`)))
  (bind _returnvalue_2 (`SceneComponent.K2_GetComponentToWorld` (`self.Lane0`)))
  (bind _returnvalue_3 (`SceneComponent.K2_GetComponentToWorld` (`self.Lane1`)))
  ;[1 1 1] Lane0
  (switch `int` (`KismetMathLibrary.RandomIntegerInRange` 0 2)
    (:`1`
      (`|SpawnActorFromClass` "/Game/MyContent/RunnerFiles/Blueprints/Obstacle.Obstacle_C" _returnvalue_2 "Undefined" "OverrideRootScale" null null)
      ;[1 1 1] Lane1
      (switch `int` (`KismetMathLibrary.RandomIntegerInRange` 0 2)
        (:`1`
          (`|SpawnActorFromClass` "/Game/MyContent/RunnerFiles/Blueprints/Obstacle.Obstacle_C" _returnvalue_3 "Undefined" "OverrideRootScale" null null)
          ;[1 1 1] Lane2
          (switch `int` (`KismetMathLibrary.RandomIntegerInRange` 0 2)
            (:`1`
              (`|SpawnActorFromClass` "/Game/MyContent/RunnerFiles/Blueprints/Obstacle.Obstacle_C" _returnvalue "Undefined" "OverrideRootScale" null null))
            (:`2`
              (`|SpawnActorFromClass` "/Game/MyContent/RunnerFiles/Blueprints/Gem_Pickup_level2.Gem_Pickup_level2_C" _returnvalue "Undefined" "OverrideRootScale" null null))))
        (:`2`
          (`|SpawnActorFromClass` "/Game/MyContent/RunnerFiles/Blueprints/Gem_Pickup_level2.Gem_Pickup_level2_C" _returnvalue_3 "Undefined" "OverrideRootScale" null null))))
    (:`2`
      (`|SpawnActorFromClass` "/Game/MyContent/RunnerFiles/Blueprints/Gem_Pickup_level2.Gem_Pickup_level2_C" _returnvalue_2 "Undefined" "OverrideRootScale" null null))))

(fn `UserConstructionScript`)